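; BP_EnemySpawner is an actor that populates the level with enemies in waves.
; On BeginPlay it gathers every BP_EnemySpawnLocation, prints the count, and gives each location an 80% chance to spawn a BP_Enemy.
; A self-calling check polls all BP_Enemy actors every two seconds through a GetAllActorsOfClass query and respawns a new wave once none remain.
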(event `self.ReceiveBeginPlay`
  (bind _outactors (`GameplayStatics.GetAllActorsOfClass` "/Game/Blueprints/BP_EnemySpawnLocation.BP_EnemySpawnLocation_C"))
  (`KismetSystemLibrary.PrintString` (`KismetStringLibrary.Concat_StrStr` "There are " (`KismetStringLibrary.Conv_IntToString` (`KismetArrayLibrary.Array_Length` _outactors)) " spawn locations") true true (struct :`G` 0.66 :`B` 1.0 :`A` 1.0) 10.0)
  (`self.Spawn Enemies`)
  (`self.Check Enemy Count`))

(event `Spawn Enemies`
  (for _array_element (stale `self.ReceiveBeginPlay` _outactors)
    (if (< (`KismetMathLibrary.RandomFloat`) 0.8)
      (`|SpawnActorFromClass` "/Game/Blueprints/BP_Enemy.BP_Enemy_C" (`self.GetTransform` _array_element) "Undefined" "MultiplyWithRoot" null null))))

(event `Check Enemy Count`
  (bind _outactors (`GameplayStatics.GetAllActorsOfClass` "/Game/Blueprints/BP_Enemy.BP_Enemy_C")) ; expensive way to check for enemies
  (if (not (> (`KismetArrayLibrary.Array_Length` _outactors) 0))
    (`self.Spawn Enemies`))
  (`KismetSystemLibrary.Delay` 2.0)
  (`self.Check Enemy Count`))

(fn `UserConstructionScript`)