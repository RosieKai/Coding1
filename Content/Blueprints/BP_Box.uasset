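; BP_Box is a box actor that keeps spawning BP_Key actors above its cube mesh.
; On BeginPlay it prints its name, the cube's world location and the raised spawn point as colored debug text.
; It then spawns a randomly scaled key at that point, waits SpawnDelay seconds and wires back to the spawn, forming an endless loop through the Delay node.
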(event `self.ReceiveBeginPlay`
  (bind _returnvalue (`SceneComponent.K2_GetComponentLocation` (`self.Cube`)))
  (bind _returnvalue_2 (+ _returnvalue (0.0 0.0 100.0)))
  (`KismetSystemLibrary.PrintString` (`KismetStringLibrary.Concat_StrStr` (`KismetSystemLibrary.GetDisplayName` self) " exists!") true true (struct :`G` 0.66 :`B` 1.0 :`A` 1.0) 10.0)
  (`KismetSystemLibrary.PrintString` (`KismetStringLibrary.Conv_VectorToString` _returnvalue) true true (struct :`R` 0.308702 :`G` 0.047517 :`B` 0.670833 :`A` 1.0) 10.0)
  (`KismetSystemLibrary.PrintString` (`KismetStringLibrary.Conv_VectorToString` _returnvalue_2) true true (struct :`R` 0.916667 :`G` 0.255903 :`B` 0.707309 :`A` 1.0) 10.0)
  (`|SpawnActorFromClass` "/Game/Blueprints/BP_Key.BP_Key_C" (`KismetMathLibrary.MakeTransform` _returnvalue_2 (struct) (`KismetMathLibrary.Conv_DoubleToVector` (`KismetMathLibrary.RandomFloatInRange` 0.001 1.0))) "Undefined" "MultiplyWithRoot" null null :!label _label)
  (`KismetSystemLibrary.Delay` (`self.Spawn Delay`))
  (goto _label))

(fn `UserConstructionScript`)